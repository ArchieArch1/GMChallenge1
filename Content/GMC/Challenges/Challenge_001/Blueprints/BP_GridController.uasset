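; BP_GridController drives the BP_ZombieGrid actors of Challenge 001, activating them progressively in random order.
; BeginPlay gathers every grid in the level, and StartGrids shuffles them, activates the first and starts a looping timer with a random interval.
; Each tick activates the next grid until the index reaches the array length; the re-rolled delay never reaches the running timer.
; StopGrids deactivates all grids but leaves timer and index untouched.
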(event Custom|StartGrids
  (bind _zombiegrids (Variables|Default|GetZombieGrids))
  (Utilities|Array|Shuffle _zombiegrids)
  (Default|GridActivated (Utilities|Array|Get(acopy) _zombiegrids (Variables|Default|GetGridsInUse)))
  (Math|Integer|IncrementInt (Variables|Default|GetGridsInUse)
    (:%20%20
      (CallFunction|ManageHandSpawn))))

(event Custom|StopGrids
  (for _array_element (Variables|Default|GetZombieGrids)
    (Default|GridDecativated _array_element)))

(event EventBeginPlay
  (bind _outactors (Actor|GetAllActorsOfClass "/Game/GMC/Challenges/Challenge_001/Blueprints/BP_ZombieGrid.BP_ZombieGrid_C"))
  (for (_array_element _array_index) _outactors
    (Utilities|Array|SetArrayElem (Variables|Default|GetZombieGrids) _array_index _array_element true)))

(fn ConstructionScript)

(fn ManageHandSpawn
  (Variables|Default|SetRandomGridTime (Math|Random|RandomFloatinRange 1.5 3.5))
  (bind _returnvalue (Utilities|Time|SetTimerbyFunctionName 0 "ActivateNewGrid" (Variables|Default|GetRandomGridTime) true))
  (Variables|Default|SetGridTimer _returnvalue))

(fn ActivateNewGrid
  ;[0 0 0] Setup new grid
  (Default|GridActivated (Utilities|Array|Get(acopy) (Variables|Default|GetZombieGrids) (Variables|Default|GetGridsInUse)))
  ;[0 0 0] Are all grids activated?
  (if (== (Variables|Default|GetGridsInUse) (Utilities|Array|Length (Variables|Default|GetZombieGrids)))
    ;[0 0 0] If true, stop timer
    (Utilities|Time|ClearandInvalidateTimerbyHandle (Variables|Default|GetGridTimer))
    (else
      ;[0 0 0] If false, continue
      (Variables|Default|SetRandomGridTime (Math|Random|RandomFloatinRange 1.0 2.0))
      (Math|Integer|IncrementInt (Variables|Default|GetGridsInUse)))))