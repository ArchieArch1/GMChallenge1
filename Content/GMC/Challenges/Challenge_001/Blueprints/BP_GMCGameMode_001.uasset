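; Game mode for GMC Challenge 001, a timed score challenge with a pre-game countdown and a win or lose ending.
; BeginPlay creates the HUD, caches the grid controller and hero, then runs a looping one-second countdown.
; StartGame starts the grids and game timer; when time expires, it stops the grids and shows end-of-game UI.
; The hero celebrates if the score, raised via IncrementScore, meets the target; otherwise it plays failure.
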(event Custom|GameTimerTick
  (CallFunction|GameCountdownTimer (stale Custom|StartGame _returnvalue)))

(event Custom|StartGame
  (Default|ToggleGameUI (Variables|Default|GetHudRef))
  (Default|StartGrids (Variables|Default|GetGridControllerRef))
  (bind _returnvalue (Utilities|Time|SetTimerbyEvent (delegate Custom|GameTimerTick) 1.0 true)))

(event Custom|EndGame
  (CallFunction|CalculateResult)
  (Default|ToggleEoGUI (Variables|Default|GetHudRef)))

(event EventBeginPlay
  (Input|SetInputModeGameOnly (Game|GetPlayerController 0))
  ;[0 0 0] Get reference to HUD
  (bind _returnvalue (UserInterface|CreateWidget "/Game/GMC/Challenges/Challenge_001/UI/WBP_HUD.WBP_HUD_C"))
  (bind _output_get (Variables|Default|SetHudRef _returnvalue))
  (UserInterface|Viewport|AddtoViewport _output_get 0)
  (Default|ToggleGameStartUI (Variables|Default|GetHudRef))
  (bind _outactors (Actor|GetAllActorsOfClass "/Game/GMC/Challenges/Challenge_001/Blueprints/BP_GridController.BP_GridController_C"))
  (Variables|Default|SetGridControllerRef (Utilities|Array|Get(acopy) _outactors))
  (bind _outactors_2 (Actor|GetAllActorsOfClass "/Game/GMC/GlobalAssets/Characters/Blueprints/BP_GMCHero.BP_GMCHero_C"))
  (Variables|Default|SetPlayerRef (Utilities|Array|Get(acopy) _outactors_2))
  (Utilities|Time|SetTimerbyFunctionName 0 "StartCountdownTimer" 1.0 true 1.0))

(fn ConstructionScript)

(fn CountdownTimer
  (params (StartingTime :type Integer))
  (if (> StartingTime 0)
    (return (- StartingTime 1))))

(fn StartCountdownTimer
  ;[0 0 0] If starting time > 0, carry on counting down
  (if (> (Variables|Default|GetStartingTime) 1)
    (Variables|Default|SetStartingTime (- (Variables|Default|GetStartingTime) 1))
    (Default|SetStartUIText (Variables|Default|GetHudRef))
    (return)
    (else
      (Utilities|Time|ClearTimerbyFunctionName 0 "StartCountdownTimer")
      (Default|ToggleGameStartUI (Variables|Default|GetHudRef))
      (CallFunction|StartGame))))

(fn GameCountdownTimer
  (params (GameTimerHandle :type Timer%20Handle%20Structure))
  ;[0 0 0] If starting time > 0, carry on counting down
  (if (> (Variables|Default|GetGameTime) 1)
    (Variables|Default|SetGameTime (- (Variables|Default|GetGameTime) 1))
    (Default|SetGameUIText (Variables|Default|GetHudRef))
    (return)
    (else
      (Utilities|Time|ClearandInvalidateTimerbyHandle GameTimerHandle)
      (Default|ToggleGameUI (Variables|Default|GetHudRef))
      (Default|StopGrids (Variables|Default|GetGridControllerRef))
      (CallFunction|EndGame))))

(fn IncrementScore
  (Variables|Default|SetCurrentScore (+ (Variables|Default|GetCurrentScore) 1))
  (Default|UpdateScoreText (Variables|Default|GetHudRef)))

(fn CalculateResult
  ;[0 0 0] Has the player won?
  (if (>= (Variables|Default|GetCurrentScore) (Variables|Default|GetTargetToWin))
    (Default|PlayCelebrate (Variables|Default|GetPlayerRef))
    (else
      (Default|PlayFailure (Variables|Default|GetPlayerRef)))))