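; Zombie hand target for GMC Challenge 001 that emerges, waits to be hit, then sinks away if missed.
; BeginPlay bumps the game mode's spawn count, plays a pitch-randomized sound, caches the montage and waits a random time before jumping to its "End" section and destroying the actor.
; OnHit plays a sound and destroys it immediately.
; A dynamic material is prepared for a hit flash, but FlashGreen is an empty stub.
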(event Custom|OnHit
  (Audio|PlaySoundatLocation "/Game/GMC/Challenges/Challenge_001/Audio/SFX/zombie_hit.zombie_hit" (Transformation|GetActorLocation) "0, 0, 0" 1.0 1.0 0.0 0 0 0)
  (Actor|DestroyActor))

(event Custom|FlashGreen)

(event EventBeginPlay
  ;[0 0 0] Tell the gamemode how many hands have spawned
  (bind _outactors (Actor|GetAllActorsOfClass "/Game/GMC/Challenges/Challenge_001/Blueprints/BP_GMCGameMode_001.BP_GMCGameMode_001_C"))
  (bind _result (Math|Integer|IncrementInt (Variables|/Game/GMC/Challenges/Challenge_001/Blueprints/BP_GMCGameMode_001.BP_GMCGameMode_001_C|GetTotalHandsSpawned (Utilities|Array|Get(acopy) _outactors)))
    (:%20%20
      (Variables|/Game/GMC/Challenges/Challenge_001/Blueprints/BP_GMCGameMode_001.BP_GMCGameMode_001_C|SetTotalHandsSpawned (Utilities|Array|Get(acopy) _outactors) _result)
      (Audio|PlaySoundatLocation "/Game/GMC/Challenges/Challenge_001/Audio/SFX/Emerge.Emerge" (Transformation|GetActorLocation) "0, 0, 0" 0.3 (Math|Random|RandomFloatinRange 0.5 1.5) 0.0 0 0 0)
      (bind _output_get (Variables|Default|SetZombieAnimInstance (Components|SkeletalMesh|GetAnimInstance (Variables|Default|GetZombieHand))))
      (Variables|Default|SetZombieMontage (Animation|Montage|GetCurrentActiveMontage _output_get))
      ;[1 1 1] Hint: Use these nodes to create the material flash when hand is hit
      (bind _returnvalue (Rendering|Material|CreateDynamicMaterialInstance (Variables|Default|GetZombieHand) 0 "/Game/GMC/Challenges/Challenge_001/Materials/Props/ZombieHand/MI_ZombieHand.MI_ZombieHand" "ZombieHandMat" :!class /Script/Engine.PrimitiveComponent))
      (Variables|Default|SetHandMat _returnvalue)
      ;[0 0 0] Generate random hand duration and skip to the "End" montage segment based on the time
      (bind _duration (CallFunction|GenerateRandomHandTime))
      (bind _output_get_2 (Variables|Default|SetHandTime _duration))
      ;;[0 0 0] Wait for hand duration
      (Utilities|FlowControl|Delay _output_get_2)
      (CallFunction|SinkHand)
      (Utilities|FlowControl|Delay 1.0)
      ;[0 0 0] Destroy if missed
      (CallFunction|DestroyHand))))

(fn ConstructionScript)

(fn GenerateRandomHandTime
  (return (Math|Random|RandomFloatinRange 0.5 3.0)))

(fn SinkHand
  (Ability|Animation|MontageJumptoSection (Variables|Default|GetZombieAnimInstance) "End" (Variables|Default|GetZombieMontage)))

(fn DestroyHand
  ;[0 0 0] Destroy if the hand was missed
  (Actor|DestroyActor))

(fn IncrementTotalHands
  (bind _gamemoderef (Variables|Default|GetGameModeRef))
  (bind _result (Math|Integer|IncrementInt (Variables|/Game/GMC/Challenges/Challenge_001/Blueprints/BP_GMCGameMode_001.BP_GMCGameMode_001_C|GetTotalHandsSpawned _gamemoderef))
    (:%20%20
      (Variables|/Game/GMC/Challenges/Challenge_001/Blueprints/BP_GMCGameMode_001.BP_GMCGameMode_001_C|SetTotalHandsSpawned _gamemoderef _result))))