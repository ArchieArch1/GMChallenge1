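; BP_ZombieGrid is a zombie hand spawner that creates BP_ZombieHand actors at its own transform while activated.
; Activation spawns a hand immediately, then starts a looping timer with a random interval, which deactivation clears.
; Each tick of the timer spawns and re-rolls RandomSpawnTime, but the running timer keeps its initial interval.
; FirstHandSpawn offers a one-in-four spawn chance but is not called in this graph.
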(event Custom|SpawnHand
  (CallFunction|HandSpawner)
  (CallFunction|RandomizeSpawnTime))

(event Custom|GridActivated
  (CallFunction|HandSpawner)
  (CallFunction|RandomizeSpawnTime)
  (bind _returnvalue (Utilities|Time|SetTimerbyEvent (delegate Custom|SpawnHand) (Variables|Default|GetRandomSpawnTime) true)))

(event Custom|GridDecativated
  (Utilities|Time|ClearandInvalidateTimerbyHandle (stale Custom|GridActivated _returnvalue)))

(fn ConstructionScript)

(fn FirstHandSpawn
  ;[0 0 0] Only spawn at the start if the random int == 3
  (bind _output_get (Variables|Default|SetFirstSpawnChance (Math|Random|RandomIntegerinRange 0 3)))
  (if (== _output_get 3)
    (Game|SpawnActorfromClass "/Game/GMC/Challenges/Challenge_001/Blueprints/BP_ZombieHand.BP_ZombieHand_C" (Transformation|GetActorTransform) "Undefined" 0 0)))

(fn HandSpawner
  (Game|SpawnActorfromClass "/Game/GMC/Challenges/Challenge_001/Blueprints/BP_ZombieHand.BP_ZombieHand_C" (Transformation|GetActorTransform) "Undefined" 0 0))

(fn RandomizeSpawnTime
  (Variables|Default|SetRandomSpawnTime (Math|Random|RandomFloatinRange 3.25 7.0))
  (return))