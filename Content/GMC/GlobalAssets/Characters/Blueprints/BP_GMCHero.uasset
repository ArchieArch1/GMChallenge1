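; BP_GMCHero is the player hero, who fights zombie hands with a weapon.
; Attack input only plays a swing sound here, while weapon collision overlaps play a hit sound on any other actor.
; Overlapped BP_ZombieHand actors receive OnHit, then the game mode increments the score.
; Celebrate and PlayerLost events spawn a camera at CamPosition, blend the view to it and loop a win or lose animation.
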(event OnComponentBeginOverlap(WeaponCollision)
  (params (OverlappedComponent :type Primitive%20Component%20Object%20Reference) (OtherActor :type Actor%20Object%20Reference) (OtherComp :type Primitive%20Component%20Object%20Reference) (OtherBodyIndex :type Integer) (bFromSweep :type Boolean) (SweepResult :type Hit%20Result%20Structure%20%28by%20ref%29))
  ;[1 1 1] Hint: Use this to determine if a Zombie Hand was hit.
  (if (!= OtherActor self)
    (Audio|PlaySoundatLocation "/Game/GMC/GlobalAssets/Audio/SFX/sword_hit.sword_hit" (Transformation|GetActorLocation OtherActor) "0, 0, 0" 1.0 1.0 0.0 0 0 0)
    (bind _asbp_zombie_hand (Utilities|Casting|CastToBP_ZombieHand OtherActor))
    (Default|OnHit _asbp_zombie_hand)
    (bind _asbp_gmcgame_mode_001 (Utilities|Casting|CastToBP_GMCGameMode_001 (Game|GetGameMode)))
    (Default|IncrementScore _asbp_gmcgame_mode_001)))

(event Custom|Celebrate
  (CallFunction|PlayCelebrate))

(event Custom|PlayerLost
  (CallFunction|PlayFailure))

(event Input|ActionEvents|InputActionAttack
  (params (Key :type Key%20Structure :default "None"))
  (:Pressed
    (Audio|PlaySound2D "/Game/GMC/GlobalAssets/Audio/SFX/swing.swing" 1.0 1.0 0.0 0 self false)))

(fn ConstructionScript)

(fn PlayCelebrate
  (bind _returnvalue (Game|SpawnActorfromClass "/Script/Engine.CameraActor" (Transformation|GetWorldTransform (Variables|Default|GetCamPosition)) "Undefined" (Game|GetPlayerController 0) 0))
  (Game|Player|SetViewTargetwithBlend (Game|GetPlayerController 0) _returnvalue 0.0 "VTBlend_Linear" 0.0 false)
  (Components|Animation|PlayAnimation (Variables|Character|GetMesh) "/Game/GMC/GlobalAssets/Characters/Animations/Anim_Win_Weapon.Anim_Win_Weapon" true))

(fn PlayFailure
  (bind _returnvalue (Game|SpawnActorfromClass "/Script/Engine.CameraActor" (Transformation|GetWorldTransform (Variables|Default|GetCamPosition)) "Undefined" (Game|GetPlayerController 0) 0))
  (Game|Player|SetViewTargetwithBlend (Game|GetPlayerController 0) _returnvalue 0.0 "VTBlend_Linear" 0.0 false)
  (Components|Animation|PlayAnimation (Variables|Character|GetMesh) "/Game/GMC/GlobalAssets/Characters/Animations/Anim_Lose.Anim_Lose" true))